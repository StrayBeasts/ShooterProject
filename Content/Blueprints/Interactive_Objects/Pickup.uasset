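; Pickup is an interactive actor that restores the player character's Warmth when touched.
; A Box overlap checks for the player character, casts it to MyCharacter and adds a fixed amount to Warmth.
; It then hides the mesh, spawns a particle system at its location and destroys itself.
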(event OnComponentBeginOverlap(Box)
  (params (OverlappedComponent :type Primitive%20Component%20Object%20Reference) (OtherActor :type Actor%20Object%20Reference) (OtherComp :type Primitive%20Component%20Object%20Reference) (OtherBodyIndex :type Integer) (bFromSweep :type Boolean) (SweepResult :type Hit%20Result%20Structure%20%28by%20ref%29))
  (bind _returnvalue (Game|GetPlayerCharacter 0))
  (if (Collision|IsOverlappingActor (Variables|Default|GetBox) _returnvalue :!class /Script/Engine.PrimitiveComponent)
    (bind _asmy_character (Utilities|Casting|CastToMyCharacter _returnvalue))
    (Variables|/Game/Blueprints/Character/MyCharacter.MyCharacter_C|SetWarmth _asmy_character (+ (Variables|/Game/Blueprints/Character/MyCharacter.MyCharacter_C|GetWarmth _asmy_character) 0.5))
    (Rendering|SetVisibility (Variables|Default|GetPickupMesh) false false)
    (Niagara|SpawnSystematLocation "/Game/Particles/PickupEmitter_System.PickupEmitter_System" (Transformation|GetActorLocation))
    (Actor|DestroyActor)))

(fn ConstructionScript)
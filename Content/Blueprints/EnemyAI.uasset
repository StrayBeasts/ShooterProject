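; Enemy AI controller that runs the EnemyTree behavior tree and feeds its blackboard.
; On BeginPlay it casts the controlled pawn to MyCharacter and copies that pawn's IsLooping flag into PathLooping.
; AI perception updates for the player character set CanSeePlayer from the stimulus result.
; A DoOnce latches HasSensedPlayer to true on the first player update, whether sensed or not.
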(event OnTargetPerceptionUpdated(AIPerception)
  (params (Actor :type Actor%20Object%20Reference) (Stimulus :type AI%20Stimulus%20Structure))
  (bind _asmy_character (Utilities|Casting|CastToMyCharacter Actor))
  (if (== _asmy_character (Game|GetPlayerCharacter 0))
    (AI|Components|Blackboard|SetValueasBool (AI|GetBlackboard 0) (Utilities|Name|MakeLiteralName "CanSeePlayer") (.bsuccessfullysensed Stimulus))
    (Utilities|FlowControl|DoOnce false
      (:Completed
        (AI|Components|Blackboard|SetValueasBool (AI|GetBlackboard 0) (Utilities|Name|MakeLiteralName "HasSensedPlayer") true)))))

(event EventBeginPlay
  (AI|RunBehaviorTree "/Game/Blueprints/EnemyTree.EnemyTree")
  (bind _asmy_character (Utilities|Casting|CastToMyCharacter (Pawn|GetControlledPawn)))
  (bind _output_get (Variables|Default|SetMyPawn _asmy_character))
  (AI|Components|Blackboard|SetValueasBool (AI|GetBlackboard 0) (Utilities|Name|MakeLiteralName "PathLooping") (Variables|/Game/Blueprints/MyCharacter.MyCharacter_C|GetIsLooping _output_get)))

(fn ConstructionScript)
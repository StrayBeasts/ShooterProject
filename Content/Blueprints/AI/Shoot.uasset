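; Behavior tree task that makes an AI-controlled MyCharacter shoot.
; On execute it casts the pawn, calls Shoot and finishes successfully at once, and on abort it calls StopShooting; a failed cast leaves the task unfinished.
; A disconnected branch holds an unused looping burst-fire pattern for one ChildType, alternating Shoot and StopShooting with delays.
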(event EventReceiveExecuteAI
  (params (OwnerController :type AI%20Controller%20Object%20Reference) (ControlledPawn :type Pawn%20Object%20Reference))
  (bind _asmy_character (Utilities|Casting|CastToMyCharacter ControlledPawn))
  (Variables|Default|SetChar _asmy_character)
  (Default|Shoot (Variables|Default|GetChar))
  (AI|BehaviorTree|FinishExecute true))

(event EventReceiveAbortAI
  (params (OwnerController :type AI%20Controller%20Object%20Reference) (ControlledPawn :type Pawn%20Object%20Reference))
  (bind _asmy_character (Utilities|Casting|CastToMyCharacter ControlledPawn))
  (Default|StopShooting _asmy_character)
  (Class|BTTaskBlueprintBase|FinishAbort))
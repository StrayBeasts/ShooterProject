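; Behavior tree task that advances an AI character's patrol path index stored in the blackboard.
; It casts the controlled pawn to MyCharacter and compares the next index against the length of its PatrolPath's PathPoints.
; If another point exists, it writes the incremented index and finishes successfully; at the last point it finishes with failure, without wrapping or resetting the index.
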(event EventReceiveExecuteAI
  (params (OwnerController :type AI%20Controller%20Object%20Reference) (ControlledPawn :type Pawn%20Object%20Reference))
  (bind _bbpathindex (Variables|Default|GetBBPathIndex))
  (bind _returnvalue (Class|BTFunctionLibrary|GetBlackboardValueasInt _bbpathindex))
  (bind _returnvalue_2 (+ _returnvalue 1))
  (bind _asmy_character (Utilities|Casting|CastToMyCharacter ControlledPawn))
  (if (<= _returnvalue_2 (- (Utilities|Array|Length (Variables|/Game/Blueprints/AI/PatrolPath.PatrolPath_C|GetPathPoints (Variables|/Game/Blueprints/Character/MyCharacter.MyCharacter_C|GetPatrolPath _asmy_character))) 1))
    (Class|BTFunctionLibrary|SetBlackboardValueasInt (Variables|Default|GetBBPathIndex) _returnvalue_2)
    (AI|BehaviorTree|FinishExecute true)
    (else
      (AI|BehaviorTree|FinishExecute false))))
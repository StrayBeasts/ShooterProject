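; Behavior tree task that picks the next world-space patrol point for an AI-controlled MyCharacter.
; It turns off controller yaw rotation on the pawn, then reads the point at the blackboard path index from the character's PatrolPath.
; That local point is transformed by the path actor's transform and written to the blackboard vector key.
; The task only finishes, with success, when the cast succeeds and the path is valid.
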(event EventReceiveExecuteAI
  (params (OwnerController :type AI%20Controller%20Object%20Reference) (ControlledPawn :type Pawn%20Object%20Reference))
  (bind _asmy_character (Utilities|Casting|CastToMyCharacter ControlledPawn))
  (Variables|/Script/Engine.Pawn|SetbUseControllerRotationYaw _asmy_character false)
  (bind _patrolpath (Variables|/Game/Blueprints/Character/MyCharacter.MyCharacter_C|GetPatrolPath _asmy_character)
    (:then
      (AI|BehaviorTree|SetBlackboardValueasVector (Variables|Default|GetBBPathVector) (Math|Transform|TransformLocation (Transformation|GetActorTransform _patrolpath) (Utilities|Array|Get(acopy) (Variables|/Game/Blueprints/AI/PatrolPath.PatrolPath_C|GetPathPoints _patrolpath) (Class|BTFunctionLibrary|GetBlackboardValueasInt (Variables|Default|GetBBPathIndex)))))
      (AI|BehaviorTree|FinishExecute true))
    (:else)))
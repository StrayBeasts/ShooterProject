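; EnemyAI is the enemy AI controller, running the EnemyTree behavior tree and feeding its blackboard.
; On BeginPlay it stores the player and the pawn's path-looping flag, then sets wait and shoot timings according to the pawn's ChildType.
; Perception updates track whether sight currently detects the player, latch first-sighting flags through a DoOnce, and flag damage stimuli as both sensed player and damaged.
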(event OnTargetPerceptionUpdated(AIPerception)
  (params (Actor :type Actor%20Object%20Reference) (Stimulus :type AI%20Stimulus%20Structure))
  (bind _returnvalue (Class|AIPerceptionSystem|GetSenseClassforStimulus Stimulus))
  (if (== _returnvalue "/Script/AIModule.AISense_Sight")
    (bind _asmy_character (Utilities|Casting|CastToMyCharacter Actor))
    (if (== _asmy_character (Game|GetPlayerCharacter 0))
      (AI|Components|Blackboard|SetValueasBool (AI|GetBlackboard 0) (Utilities|Name|MakeLiteralName "CanSeePlayer") (.bSuccessfullySensed (Utilities|Struct|BreakAIStimulus Stimulus)))
      (Utilities|FlowControl|DoOnce false
        (:Completed
          (AI|Components|Blackboard|SetValueasBool (AI|GetBlackboard 0) (Utilities|Name|MakeLiteralName "HasSensedPlayer") true)
          (AI|Components|Blackboard|SetValueasBool (AI|GetBlackboard 0) (Utilities|Name|MakeLiteralName "HasSeenPlayer") true))))
    (elif (== _returnvalue "/Script/AIModule.AISense_Damage")
      (AI|Components|Blackboard|SetValueasBool (AI|GetBlackboard 0) (Utilities|Name|MakeLiteralName "HasSensedPlayer") true)
      (AI|Components|Blackboard|SetValueasBool (AI|GetBlackboard 0) (Utilities|Name|MakeLiteralName "IsDamaged") true))))

(event Custom|Threatened)

(event EventBeginPlay
  (AI|RunBehaviorTree "/Game/Blueprints/AI/EnemyTree.EnemyTree")
  (bind _asmy_character (Utilities|Casting|CastToMyCharacter (Pawn|GetControlledPawn)))
  (bind _output_get (Variables|Default|SetMyPawn _asmy_character))
  (AI|Components|Blackboard|SetValueasBool (AI|GetBlackboard 0) (Utilities|Name|MakeLiteralName "PathLooping") (Variables|/Game/Blueprints/Character/MyCharacter.MyCharacter_C|GetIsLooping _output_get))
  (AI|Components|Blackboard|SetValueasObject (AI|GetBlackboard 0) (Utilities|Name|MakeLiteralName "Player") (Game|GetPlayerCharacter 0))
  (switch int (Variables|/Game/Blueprints/Character/MyCharacter.MyCharacter_C|GetChildType (Variables|Default|GetMyPawn))
    (:1
      (AI|Components|Blackboard|SetValueasFloat (AI|GetBlackboard 0) (Utilities|Name|MakeLiteralName "WaitTime") 0.4)
      (AI|Components|Blackboard|SetValueasFloat (AI|GetBlackboard 0) (Utilities|Name|MakeLiteralName "ShootTime") 3e+01))
    (:2
      (AI|Components|Blackboard|SetValueasFloat (AI|GetBlackboard 0) (Utilities|Name|MakeLiteralName "WaitTime") 0.8)
      (AI|Components|Blackboard|SetValueasFloat (AI|GetBlackboard 0) (Utilities|Name|MakeLiteralName "ShootTime") 0.1))
    (:3
      (AI|Components|Blackboard|SetValueasFloat (AI|GetBlackboard 0) (Utilities|Name|MakeLiteralName "WaitTime") 1.2)
      (AI|Components|Blackboard|SetValueasFloat (AI|GetBlackboard 0) (Utilities|Name|MakeLiteralName "ShootTime") 0.1))))

(fn ConstructionScript)
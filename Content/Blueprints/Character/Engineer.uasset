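; Engineer character Blueprint that adds hitscan shooting on top of its parent class and halves damage when not player-controlled (not player character 0).
; Shoot plays audio, first-person montage, camera shake and muzzle effect for the player, or a separate muzzle for others.
; A camera-forward line trace damages living MyCharacter targets, spawning blood on non-player victims.
; A Fired flag and Period delay limit the fire rate.
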(event EventBeginPlay
  (|CallParentFunction)
  (if (not (== self (Game|GetPlayerCharacter 0)))
    (Variables|Default|Setdamage (/ (Variables|Default|Getdamage) 2.0))))

(event EventTick
  (params (DeltaSeconds :type Float%20%28single-precision%29))
  (|CallParentFunction DeltaSeconds))

(event EventShoot
  (bind _camera_main (Variables|Default|GetCamera_main))
  (bind _returnvalue (Transformation|GetWorldLocation _camera_main))
  (if (not (Variables|Default|Getfired))
    (Components|Activation|Activate (Variables|Default|GetAudio) true)
    (if (== self (Game|GetPlayerCharacter 0))
      (Camera|PlayWorldCameraShake "/Game/Blueprints/NewCameraShake.NewCameraShake_C" (Transformation|GetActorLocation) 0.0 5e+02)
      (Animation|Montage|MontagePlay (Components|SkeletalMesh|GetAnimInstance (Variables|Default|GetMesh_fp)) "/Game/FirstPerson/Animations/FirstPersonFire_Montage.FirstPersonFire_Montage" 1.0 "MontageLength" 0.0 true)
      (Components|Activation|Activate (Variables|Default|GetMuzzlePlayer) true)
      (else
        (Components|Activation|Activate (Variables|Default|GetMuzzle) true)))
    (bind _outhit (Collision|LineTraceByChannel _returnvalue (+ _returnvalue (* (Math|Vector|GetForwardVector _camera_main) (Variables|Default|GetWeaponRange))) "TraceTypeQuery1" false 0 "None"))
    (Variables|Default|Setfired true)
    (bind _asmy_character (Utilities|Casting|CastToMyCharacter (.HitActor (Collision|BreakHitResult _outhit)))
      (:then
        (if (Variables|/Game/Blueprints/Character/MyCharacter.MyCharacter_C|GetDead _asmy_character)
          _
          (else
            (Game|Damage|ApplyDamage (.HitActor (Collision|BreakHitResult _outhit)) (Variables|Default|Getdamage) 0 self "/Game/Blueprints/DamageTypes/Shoot.Shoot_C")
            (if (!= (.HitActor (Collision|BreakHitResult _outhit)) (Game|GetPlayerCharacter 0))
              (Niagara|SpawnSystematLocation "/Game/Particles/BloodEmitter_System.BloodEmitter_System" (.ImpactPoint (Collision|BreakHitResult _outhit)) (Math|Rotator|MakeRotator (Math|Random|RandomFloatinRange -45.0 45.0) 0.0 0.0))))))
      (:CastFailed
        _))
    (Utilities|FlowControl|Delay (Variables|Default|Getperiod))
    (Variables|Default|Setfired false)))

(event EventStopShooting)

(fn ConstructionScript
  (|CallParentFunction))